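; Dilo is an AI pawn that roams the navmesh and reacts when it sees the player character.
; Every Tick it requests a simple move to a random point up to 5000 units away, projected onto the navmesh.
; PawnSensing sightings of a ThirdPersonCharacter print a debug message and request a move to that actor, which the next Tick's random move replaces.
; Alternative chase, stop and material-colour nodes are left unconnected.
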(event `self.PawnSensing.OnSeePawn`
  (params (Pawn :type "Pawn Object Reference"))
  (bind _asthird_person_character (cast `/Game/MyContent/Blueprints/ThirdPersonCharacter` Pawn))
  (`KismetSystemLibrary.PrintString` "Hello")
  (`NavigationSystem.SimpleMoveToActor` (`AIBlueprintHelperLibrary.GetAIController` self) _asthird_person_character))

(event `self.ReceiveTick`
  (params (DeltaSeconds :type "Float (single-precision)"))
  ;[1 1 1] Moves pawn toward player
  (bind _asaicontroller (cast `AIController` (`self.GetController`)))
  (`NavigationSystem.SimpleMoveToLocation` _asaicontroller (`NavigationSystem.K2_ProjectPointToNavigation` (+ (`self.K2_GetActorLocation`) (* (`KismetMathLibrary.RandomUnitVector`) 5000.0)) null null (0.0 0.0 5000.0))))

(fn `UserConstructionScript`)